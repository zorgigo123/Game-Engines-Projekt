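; AI_BP is an enemy AI pawn that wanders around its spawn point, targets the player on sight and damages them on contact.
; At BeginPlay it writes its roaming range and start location to the Blackboard.
; PawnSensing stores the first sighting of the player as the Blackboard Enemy.
; Hitting the player applies damage through MyPawn, teleports the AI to its start and clears the enemy, resetting the cycle.
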(event `self.ReceiveBeginPlay`
  (set `self.StartLocation` (`self.K2_GetActorLocation`))
  (`BlackboardComponent.SetValueAsFloat` (`AIBlueprintHelperLibrary.GetBlackboard` (`AIBlueprintHelperLibrary.GetAIController` self)) "RoamingRange" (`self.MaxWanderDistance`))
  (`BlackboardComponent.SetValueAsVector` (`AIBlueprintHelperLibrary.GetBlackboard` (`AIBlueprintHelperLibrary.GetAIController` self)) "StartLocation" (`self.StartLocation`)))

(event `self.PawnSensing.OnSeePawn`
  (params (Pawn :type "Pawn Object Reference"))
  (if (== Pawn (`GameplayStatics.GetPlayerPawn` 0))
    (`/Engine/EditorBlueprintResources/StandardMacros.IsValid` (`self.EnemyPawn`)
      (:`Is Not Valid`
        (bind _output_get (set `self.EnemyPawn` Pawn))
        (`BlackboardComponent.SetValueAsObject` (`AIBlueprintHelperLibrary.GetBlackboard` (`AIBlueprintHelperLibrary.GetAIController` self)) "Enemy" _output_get)))))

(event `self.ReceiveHit`
  (params (MyComp :type "PrimitiveComponent Object Reference") (Other :type "Actor Object Reference") (OtherComp :type "PrimitiveComponent Object Reference") (bSelfMoved :type Boolean) (HitLocation :type "Vector Structure") (HitNormal :type "Vector Structure") (NormalImpulse :type "Vector Structure") (Hit :type "HitResult Structure (by ref)"))
  (bind _returnvalue (`GameplayStatics.GetPlayerPawn` 0))
  (if (== Other _returnvalue)
    (bind _asmy_pawn (cast `/Game/PlayerCHaracter/MyPawn` _returnvalue))
    (`/Game/PlayerCHaracter/MyPawn.DoDamage` _asmy_pawn 50.0)
    (`self.K2_SetActorLocation` (`self.StartLocation`))
    (set `self.EnemyPawn` null)
    (`BlackboardComponent.ClearValue` (`AIBlueprintHelperLibrary.GetBlackboard` (`AIBlueprintHelperLibrary.GetAIController` self)) "Enemy")))

(fn `UserConstructionScript`)