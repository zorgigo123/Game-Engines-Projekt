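; Slot-based inventory that stacks, drags, transfers, throws and uses items, with per-type stack limits and classes from a ReferenceList map.
; PickUpSlot tops up matching stacks, then fills free slots and returns any leftover.
; DragSlot buffers an amount for dropping (merge or swap), sending to another inventory, returning, or spawning as a dropped actor.
; UseSlot constructs and runs the item's use object, but reads type and count from slot 0, not Index.
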(event `self.ReceiveBeginPlay`
  (if (< (`KismetArrayLibrary.Array_Length` (`self.Slots`)) (`self.MaxSlots`))
    (`KismetArrayLibrary.Array_Set` (`self.Slots`) (- (`self.MaxSlots`) 1) (make `/Game/Inventory/SystemBase/Structures/InventorySlotStructure` "") true)))

(fn `DragSlot`
  (params (Index :type Integer) (Amount :type Integer))
  (bind (_output_itemname _output_type _output_amouunt) (break `/Game/Inventory/SystemBase/Structures/InventorySlotStructure` (`|GetArrayItem` (`self.Slots`) Index)))
  (bind _returnvalue (- _output_amouunt Amount))
  (set `self.OriginalIndex` Index)
  (set `self.DragedSlot` (make `/Game/Inventory/SystemBase/Structures/InventorySlotStructure` _output_itemname _output_type Amount))
  (if (== _returnvalue 0)
    (`KismetArrayLibrary.Array_Set` (`self.Slots`) (`self.OriginalIndex`) (make `/Game/Inventory/SystemBase/Structures/InventorySlotStructure` "") true)
    (else
      (`KismetArrayLibrary.Array_Set` (`self.Slots`) (`self.OriginalIndex`) (make `/Game/Inventory/SystemBase/Structures/InventorySlotStructure` _output_itemname _output_type _returnvalue) true))))

(fn `DropSlot`
  (params (Index :type Integer))
  (bind (_dragedslot_itemname _dragedslot_type) (break `/Game/Inventory/SystemBase/Structures/InventorySlotStructure` (`self.DragedSlot`)))
  (bind _referencelist_map (break `/Game/Inventory/SystemBase/Structures/ItemReferenceMap` (`self.ReferenceList`)))
  (bind (_dragedslot_itemname_2 _dragedslot_type_2 _dragedslot_amouunt) (break `/Game/Inventory/SystemBase/Structures/InventorySlotStructure` (`self.DragedSlot`)))
  (bind (_output_itemname _output_type _output_amouunt) (break `/Game/Inventory/SystemBase/Structures/InventorySlotStructure` (`|GetArrayItem` (`self.Slots`) Index)))
  (bind _returnvalue (+ _output_amouunt _dragedslot_amouunt))
  (if (`|EnumEquality` _output_type "NewEnumerator0")
    (`KismetArrayLibrary.Array_Set` (`self.Slots`) Index (`self.DragedSlot`) true)
    (set `self.DragedSlot` (make `/Game/Inventory/SystemBase/Structures/InventorySlotStructure` "") :!label _label)
    (set `self.OriginalIndex` -1)
    (elif (`|EnumEquality` _output_type _dragedslot_type_2)
      (if (>= (`.MaxAmount_13_092E97334399504451D72FAFDE887119` (break `/Game/Inventory/SystemBase/Structures/ItemSlotStructure` (`BlueprintMapLibrary.Map_Find` _referencelist_map _dragedslot_type_2))) _returnvalue)
        (`KismetArrayLibrary.Array_Set` (`self.Slots`) Index (make `/Game/Inventory/SystemBase/Structures/InventorySlotStructure` _dragedslot_itemname _dragedslot_type _returnvalue) true)
        (goto _label)
        (else
          (`self.ReturnSlot`)))
      (else
        (`KismetArrayLibrary.Array_Set` (`self.Slots`) (`self.OriginalIndex`) (`|GetArrayItem` (`self.Slots`) Index) true)
        (`KismetArrayLibrary.Array_Set` (`self.Slots`) Index (`self.DragedSlot`))
        (goto _label)))))

(fn `GetInventorySlots`
  (returns (Slots :type "Array of /Game/Inventory/SystemBase/Structures/InventorySlotStructure Structure"))
  (return (`self.Slots`)))

(fn `PickUpSlot`
  (params (Slot :type "/Game/Inventory/SystemBase/Structures/InventorySlotStructure Structure"))
  (returns (Return :type Boolean) (AmountLeft :type Integer))
  (locals (Added :type Boolean) (Proxy :type "/Game/Inventory/SystemBase/Structures/InventorySlotStructure Structure") (SavedAmount :type Integer) (SavedAmountProxy :type Integer))
  (bind (_proxy_itemname _proxy_type) (break `/Game/Inventory/SystemBase/Structures/InventorySlotStructure` (`local.Proxy`)))
  (bind _referencelist_map (break `/Game/Inventory/SystemBase/Structures/ItemReferenceMap` (`self.ReferenceList`)))
  (bind (_proxy_itemname_2 _proxy_type_2) (break `/Game/Inventory/SystemBase/Structures/InventorySlotStructure` (`local.Proxy`)))
  (bind _referencelist_map_2 (break `/Game/Inventory/SystemBase/Structures/ItemReferenceMap` (`self.ReferenceList`)))
  (bind _savedamount (`local.SavedAmount`))
  (bind (_proxy_itemname_3 _proxy_type_3) (break `/Game/Inventory/SystemBase/Structures/InventorySlotStructure` (`local.Proxy`)))
  (bind (_itemname _type) (break `/Game/Inventory/SystemBase/Structures/InventorySlotStructure` (`local.Proxy`)))
  (bind _returnvalue (`KismetArrayLibrary.Array_Find` (`self.Slots`)))
  (bind _value (`BlueprintMapLibrary.Map_Find` _referencelist_map_2 _proxy_type_2))
  (bind _value_2 (`BlueprintMapLibrary.Map_Find` _referencelist_map _type))
  (bind _returnvalue_2 (select `bool` (> _savedamount (`.MaxAmount_13_092E97334399504451D72FAFDE887119` (break `/Game/Inventory/SystemBase/Structures/ItemSlotStructure` _value))) :`false` _savedamount :`true` (`.MaxAmount_13_092E97334399504451D72FAFDE887119` (break `/Game/Inventory/SystemBase/Structures/ItemSlotStructure` _value))))
  (bind _output_get (set `local.Proxy` Slot))
  (set `local.SavedAmount` (`.Amouunt_8_6293F01446DF87AB9994ECAD106050C4` (break `/Game/Inventory/SystemBase/Structures/InventorySlotStructure` _output_get)))
  (for (_array_element _array_index) (`self.Slots`) :!label _label
    (bind (_itemname_2 _type_2 _amouunt) (break `/Game/Inventory/SystemBase/Structures/InventorySlotStructure` _array_element))
    (if (and (`|EnumEquality` _type_2 _type) (< _amouunt (`.MaxAmount_13_092E97334399504451D72FAFDE887119` (break `/Game/Inventory/SystemBase/Structures/ItemSlotStructure` _value_2))))
      (set `local.SavedAmountProxy` (`local.SavedAmount`))
      (bind _returnvalue_3 (- (`.MaxAmount_13_092E97334399504451D72FAFDE887119` (break `/Game/Inventory/SystemBase/Structures/ItemSlotStructure` _value_2)) _amouunt))
      (bind _returnvalue_4 (> (`local.SavedAmountProxy`) _returnvalue_3))
      (set `local.SavedAmount` (`KismetMathLibrary.SelectInt` (- (`local.SavedAmount`) _returnvalue_3) 0 _returnvalue_4))
      (`KismetArrayLibrary.Array_Set` (`self.Slots`) _array_index (make `/Game/Inventory/SystemBase/Structures/InventorySlotStructure` _proxy_itemname _proxy_type (`KismetMathLibrary.SelectInt` (`.MaxAmount_13_092E97334399504451D72FAFDE887119` (break `/Game/Inventory/SystemBase/Structures/ItemSlotStructure` _value_2)) (+ _amouunt (`local.SavedAmountProxy`)) _returnvalue_4)) true)
      (set `local.Added` true)
      (break)))
  (if (and (> (`local.SavedAmount`) 0) (`local.Added`))
    (set `local.Added` false)
    (goto _label)
    (elif (`local.Added`)
      (return true 0)
      (else
        (if (!= _returnvalue -1) :!label _label_2
          (`KismetArrayLibrary.Array_Set` (`self.Slots`) _returnvalue (make `/Game/Inventory/SystemBase/Structures/InventorySlotStructure` _proxy_itemname_3 _proxy_type_3 _returnvalue_2) true)
          (bind _output_get_2 (set `local.SavedAmount` (- (`local.SavedAmount`) _returnvalue_2)))
          (if (> _output_get_2 0)
            (goto _label_2)
            (else
              (return true 0)))
          (else
            (return false (`local.SavedAmount`))))))))

(fn `ReceiveSlot`
  (params (Index :type Integer) (Slot :type "/Game/Inventory/SystemBase/Structures/InventorySlotStructure Structure"))
  (returns (Return :type Boolean))
  (bind (_itemname _type) (break `/Game/Inventory/SystemBase/Structures/InventorySlotStructure` Slot))
  (bind (_itemname_2 _type_2 _amouunt) (break `/Game/Inventory/SystemBase/Structures/InventorySlotStructure` Slot))
  (bind _referencelist_map (break `/Game/Inventory/SystemBase/Structures/ItemReferenceMap` (`self.ReferenceList`)))
  (bind (_output_itemname _output_type _output_amouunt) (break `/Game/Inventory/SystemBase/Structures/InventorySlotStructure` (`|GetArrayItem` (`self.Slots`) Index)))
  (bind _returnvalue (+ _output_amouunt _amouunt))
  (if (`|EnumEquality` _output_type "NewEnumerator0")
    (`KismetArrayLibrary.Array_Set` (`self.Slots`) Index Slot true)
    (elif (`|EnumEquality` _output_type _type_2)
      (if (>= (`.MaxAmount_13_092E97334399504451D72FAFDE887119` (break `/Game/Inventory/SystemBase/Structures/ItemSlotStructure` (`BlueprintMapLibrary.Map_Find` _referencelist_map _type_2))) _returnvalue)
        (`KismetArrayLibrary.Array_Set` (`self.Slots`) Index (make `/Game/Inventory/SystemBase/Structures/InventorySlotStructure` _itemname _type _returnvalue) true)
        (else
          (return false)))
      (else
        (return false))))
  (return true))

(fn `ReturnSlot`
  (bind (_dragedslot_itemname _dragedslot_type _dragedslot_amouunt) (break `/Game/Inventory/SystemBase/Structures/InventorySlotStructure` (`self.DragedSlot`)))
  (bind _slots (`self.Slots`))
  (bind _originalindex (`self.OriginalIndex`))
  (bind (_dragedslot_itemname_2 _dragedslot_type_2) (break `/Game/Inventory/SystemBase/Structures/InventorySlotStructure` (`self.DragedSlot`)))
  (bind (_output_itemname _output_type _output_amouunt) (break `/Game/Inventory/SystemBase/Structures/InventorySlotStructure` (`|GetArrayItem` (`self.Slots`) (`self.OriginalIndex`))))
  (bind (_output_itemname_2 _output_type_2) (break `/Game/Inventory/SystemBase/Structures/InventorySlotStructure` (`|GetArrayItem` (`self.Slots`) (`self.OriginalIndex`))))
  (if (`|EnumEquality` _output_type_2 _dragedslot_type_2)
    (`KismetArrayLibrary.Array_Set` _slots _originalindex (make `/Game/Inventory/SystemBase/Structures/InventorySlotStructure` _output_itemname _output_type (+ _output_amouunt _dragedslot_amouunt)) true)
    (else
      (`KismetArrayLibrary.Array_Set` _slots _originalindex (make `/Game/Inventory/SystemBase/Structures/InventorySlotStructure` _dragedslot_itemname _dragedslot_type _dragedslot_amouunt) true)))
  (set `self.OriginalIndex` -1)
  (set `self.DragedSlot` (make `/Game/Inventory/SystemBase/Structures/InventorySlotStructure` "")))

(fn `SendSlot`
  (params (To :type "Object Object Reference") (Index :type Integer))
  (bind _return (message `/Game/Inventory/Blueprints/Inventory_Inteface.ReceiveSlot` To Index (`self.DragedSlot`)))
  (if _return
    (set `self.DragedSlot` (make `/Game/Inventory/SystemBase/Structures/InventorySlotStructure` ""))
    (set `self.OriginalIndex` -1)
    (else
      (`self.ReturnSlot`))))

(fn `ThrowSlot`
  (params (Location :type "Vector Structure") (Vector :type "Vector Structure"))
  (bind _referencelist_map (break `/Game/Inventory/SystemBase/Structures/ItemReferenceMap` (`self.ReferenceList`)))
  (bind (_dragedslot_itemname _dragedslot_type) (break `/Game/Inventory/SystemBase/Structures/InventorySlotStructure` (`self.DragedSlot`)))
  (`|SpawnActorFromClass` (`|ConvertAsset` (`.DropClass_15_030599594AAE16F115E48B864263AE70` (break `/Game/Inventory/SystemBase/Structures/ItemSlotStructure` (`BlueprintMapLibrary.Map_Find` _referencelist_map _dragedslot_type)))) (`KismetMathLibrary.MakeTransform` (+ Location (* Vector 200.0))) "Undefined" "MultiplyWithRoot" null (`self.DragedSlot`) null)
  (set `self.DragedSlot` (make `/Game/Inventory/SystemBase/Structures/InventorySlotStructure` ""))
  (set `self.OriginalIndex` -1))

(fn `UseSlot`
  (params (Index :type Integer))
  (bind _slots (`self.Slots`))
  (bind _referencelist_map (break `/Game/Inventory/SystemBase/Structures/ItemReferenceMap` (`self.ReferenceList`)))
  (bind (_output_itemname _output_type _output_amouunt) (break `/Game/Inventory/SystemBase/Structures/InventorySlotStructure` (`|GetArrayItem` (`self.Slots`))))
  (bind (_output_itemname_2 _output_type_2 _output_amouunt_2) (break `/Game/Inventory/SystemBase/Structures/InventorySlotStructure` (`|GetArrayItem` (`self.Slots`) Index)))
  (bind _returnvalue (`|GenericCreateObject` (`KismetSystemLibrary.GetOuterObject` self) (`|ConvertAsset` (break `/Game/Inventory/SystemBase/Structures/ItemSlotStructure` (`BlueprintMapLibrary.Map_Find` _referencelist_map _output_type)))))
  (`/Game/Items/Base/UseFunction_Base.Use` _returnvalue)
  (if (> (- _output_amouunt 1) 0)
    (`KismetArrayLibrary.Array_Set` _slots Index (make `/Game/Inventory/SystemBase/Structures/InventorySlotStructure` _output_itemname_2 _output_type_2 (- _output_amouunt_2 1)) true)
    (else
      (`KismetArrayLibrary.Array_Set` _slots Index (make `/Game/Inventory/SystemBase/Structures/InventorySlotStructure` "") true))))